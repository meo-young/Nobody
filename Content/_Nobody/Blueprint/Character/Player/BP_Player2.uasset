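; Player character Blueprint that stages death jumpscares for Doll and Mannequin types.
; BeginPlay builds the body with a runtime skeletal mesh merge and adds blur and blood overlay widgets.
; ShowDeadJumpScare plays the matching sequence, while Sequencer event endpoints trigger overlay animations and 2D scare and blood sounds.
; Tick copies the scream and anger values into morph targets on the doll jumpscare mesh.
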(event `self.ReceiveBeginPlay`
  (bind _returnvalue (`SkeletalMergingLibrary.MergeMeshes` (`self.Params`)))
  (`SkeletalMeshComponent.SetSkeletalMeshAsset` (`self.Mesh`) _returnvalue)
  (bind _returnvalue_2 (`|CreateWidget` "/Game/_Nobody/UI/WBP_Blur.WBP_Blur_C"))
  (bind _output_get (set `self.BlurUI` _returnvalue_2))
  (`UserWidget.AddToViewport` _output_get 0)
  (bind _returnvalue_3 (`|CreateWidget` "/Game/_Nobody/UI/WBP_Blood.WBP_Blood_C"))
  (bind _output_get_2 (set `self.BloodUI` _returnvalue_3))
  (`UserWidget.AddToViewport` _output_get_2 0))

(event `self.ReceiveTick`
  (params (DeltaSeconds :type "Float (single-precision)"))
  (`SkeletalMeshComponent.SetMorphTarget` (`self.DollJumpScareMesh`) "Scream" (`self.InScreamValue`) true)
  (`SkeletalMeshComponent.SetMorphTarget` (`self.DollJumpScareMesh`) "AngryPain" (`self.InAngryValue`) true))

(event `self.ShowDeadJumpScare`
  (params (JumpScareType :type "EJumpScareType Enum" :default "Doll"))
  (switch `EJumpScareType` JumpScareType
    (:`Doll`
      (`ActorSequenceComponent.PlaySequence` (`self.Doll JumpScare Sequence`)))
    (:`Mannequin`
      (`ActorSequenceComponent.PlaySequence` (`self.Mannequin JumpScare Sequence`)))))

(event `Owner_Event`
  (params (Owner :type "Actor Object Reference"))
  (bind _bloodui (`self.BloodUI`))
  (`UserWidget.PlayAnimation` _bloodui (`/Game/_Nobody/UI/WBP_Blood.ShowBlood` _bloodui) 0.0 1 "Forward" 1.0 false))

(event `Owner_Event_0`
  (params (Owner :type "Actor Object Reference"))
  (bind _blurui (`self.BlurUI`))
  (`UserWidget.PlayAnimation` _blurui (`/Game/_Nobody/UI/WBP_Blur.ShowBlur` _blurui) 0.0 1 "Forward" 1.0 false))

(event `Owner_Event_1`
  (params (Owner :type "Actor Object Reference"))
  (`GameplayStatics.PlaySound2D` "/Game/All_In_One_HorrorGame_v1/Stereo/Jumpscare/Audio/Jumpscare_People_Toys_Stereo.Jumpscare_People_Toys_Stereo" 1.0 1.0 0.0 null null))

(event `Owner_Event_2`
  (params (Owner :type "Actor Object Reference"))
  (`GameplayStatics.PlaySound2D` "/Game/_Nobody/Sound/Blood/SC_Blood1.SC_Blood1" 1.0 1.0 0.0 null null))

(event `Owner_Event_3`
  (params (Owner :type "Actor Object Reference"))
  (`GameplayStatics.PlaySound2D` "/Game/_Nobody/Sound/Blood/SC_Blood2.SC_Blood2" 1.0 1.0 0.0 null null))

(event `Owner_Event_4`
  (params (Owner :type "Actor Object Reference"))
  (`GameplayStatics.PlaySound2D` "/Game/All_In_One_HorrorGame_v1/Stereo/Jumpscare/Cue/Jumpscare_The_Crazies_Stereo_Cue.Jumpscare_The_Crazies_Stereo_Cue" 1.0 1.0 0.0 null null false))

(event `Owner_Event_6`
  (params (Owner :type "Actor Object Reference"))
  (bind _bloodui (`self.BloodUI`))
  (`UserWidget.PlayAnimation` _bloodui (`/Game/_Nobody/UI/WBP_Blood.ShowBlood` _bloodui) 0.0 1 "Forward" 1.0 false))

(event `Owner_Event_5`
  (params (Owner :type "Actor Object Reference"))
  (bind _blurui (`self.BlurUI`))
  (`UserWidget.PlayAnimation` _blurui (`/Game/_Nobody/UI/WBP_Blur.ShowBlur` _blurui) 0.0 1 "Forward" 1.0 false))

(event `Owner_Event_7`
  (params (Owner :type "Actor Object Reference"))
  (`GameplayStatics.PlaySound2D` "/Game/_Nobody/Sound/Blood/SC_Blood3.SC_Blood3" 1.0 1.0 0.0 null null))

(event `Owner_Event_8`
  (params (Owner :type "Actor Object Reference"))
  (`GameplayStatics.PlaySound2D` "/Game/_Nobody/Sound/Blood/SC_Blood1.SC_Blood1" 1.0 1.0 0.0 null null))

(fn `UserConstructionScript`)