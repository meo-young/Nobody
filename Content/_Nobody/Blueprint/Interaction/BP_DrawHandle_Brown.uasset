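; BP_DrawHandle_Brown is an interactable drawer handle that plays open and close actions with matching sounds.
; The interaction start and end events each play their own sequence, StartSequence or EndSequence, and a drawer sound cue at the actor's location.
; Sequencer event endpoints call OnStartActorSequenceEnded and OnEndActorSequenceEnded to report when each sequence ends.
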(event `self.PlayInteractionStartSequence`
  (`ActorSequenceComponent.PlaySequence` (`self.StartSequence`))
  (`GameplayStatics.PlaySoundAtLocation` "/Game/_Nobody/Sound/Drawer/Drawer_Open_Cue.Drawer_Open_Cue" (`self.K2_GetActorLocation`) (struct) 1.0 1.0 0.0 null null null null))

(event `self.PlayInteractionEndSequence`
  (`ActorSequenceComponent.PlaySequence` (`self.EndSequence`))
  (`GameplayStatics.PlaySoundAtLocation` "/Game/_Nobody/Sound/Drawer/Drawer_Close_Cue.Drawer_Close_Cue" (`self.K2_GetActorLocation`) (struct) 1.0 1.0 0.0 null null null null))

(event `Owner_Event_1`
  (params (Owner :type "Actor Object Reference"))
  (`self.OnStartActorSequenceEnded`))

(event `Owner_Event_2`
  (params (Owner :type "Actor Object Reference"))
  (`self.OnEndActorSequenceEnded`))

(fn `UserConstructionScript`)