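; BP_OpenableDoor is an interactable door that opens and closes through two actor sequences.
; The interaction start and end events play the open and close sequences.
; Sequencer event endpoints report each sequence's completion back to the interaction logic, play door open and close sounds at the actor's location, and trigger an event-activation check.
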(event `self.PlayInteractionStartSequence`
  (`ActorSequenceComponent.PlaySequence` (`self.OpenDoorActorSequence`)))

(event `self.PlayInteractionEndSequence`
  (`ActorSequenceComponent.PlaySequence` (`self.CloseDoorActorSequence`)))

(event `OnOpenDoor`
  (`self.OnStartActorSequenceEnded`))

(event `OnCloseDoor`
  (`self.OnEndActorSequenceEnded`))

(event `PlayDoorknobSound`
  (`SoundLibrary.PlaySFXInLocation` self "Door_Open" (`self.K2_GetActorLocation`)))

(event `SequenceEvent`
  (`SoundLibrary.PlaySFXInLocation` self "Door_Close" (`self.K2_GetActorLocation`)))

(event `SequenceEvent_0`
  (`self.CheckIfEventActivated`))

(fn `UserConstructionScript`)