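; BP_OpenableDoor1 is an interactable door that opens and closes through actor sequences.
; Interaction start and end events play the open and close sequences respectively.
; Sequencer events call back to report each sequence's end, play open or close sounds at the door's location, and call CheckIfEventActivated.
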(event `self.PlayInteractionStartSequence`
  (`ActorSequenceComponent.PlaySequence` (`self.OpenDoorActorSequence`)))

(event `self.PlayInteractionEndSequence`
  (`ActorSequenceComponent.PlaySequence` (`self.CloseDoorActorSequence`)))

(event `SequenceEvent`
  (`self.OnStartActorSequenceEnded`))

(event `SequenceEvent_0`
  (`self.OnEndActorSequenceEnded`))

(event `PlayDoorSound`
  (`SoundLibrary.PlaySFXInLocation` self "Door_Open" (`self.K2_GetActorLocation`)))

(event `SequenceEvent_1`
  (`SoundLibrary.PlaySFXInLocation` self "Door_Close" (`self.K2_GetActorLocation`)))

(event `SequenceEvent_2`
  (`self.CheckIfEventActivated`))

(fn `UserConstructionScript`)